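; Souls-like player character that spawns an equipped weapon and handles movement, combat, damage, death and bonfire interaction.
; Tick drives boss lock-on rotation and distance-pitched camera, backstep movement, hold-to-run and the death state change.
; Input plays montages for roll/backstep, combo attacks, critical hits on groggy bosses, block, parry and drinking.
; Bonfire rest triggers a level reset through the game mode, whose reset event restores HP and Estus.
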(event `self.ReceiveBeginPlay`
  (bind _returnvalue (`self.GetOwner`))
  (`|ExecutionSequence`
    (:`then_0`
      (bind _returnvalue_2 (`GameplayStatics.GetActorOfClass` "/Game/Stuff/bonfire/BP_Bonfire.BP_Bonfire_C"))
      (set `self.BonfireActor` _returnvalue_2)
      (set `self.CurrentHP` (`self.MaxHP`))
      (set `self.EstusAmount` (`self.MaxEstusAmount`))
      ; Attach Weapon
      (bind _returnvalue_3 (`|SpawnActorFromClass` "/Game/Player/Weapon/BP_Weapon.BP_Weapon_C" (`SceneComponent.GetSocketTransform` (`self.Mesh`) "weapon_handgrip_r" "RTS_World") "Undefined" "MultiplyWithRoot" self null))
      (bind _output_get (set `self.EquippedWeapon` _returnvalue_3))
      (`self.K2_AttachToComponent` _output_get (`self.Mesh`) "weapon_handgrip_r" "SnapToTarget" "SnapToTarget" "SnapToTarget" true)
      (bind _asbp_soul_game_mode_level_and_state (cast `/Game/Blueprints/BP_SoulGameMode_LevelAndState` (`GameplayStatics.GetGameMode`)))
      (add `/Game/Blueprints/BP_SoulGameMode_LevelAndState.ResetBossLevel` _asbp_soul_game_mode_level_and_state (delegate `/Game/Utility/BPI_OnOff.Activate`)))
    (:`then_1`
      (`/Engine/EditorBlueprintResources/StandardMacros.IsValid` _returnvalue
        (:`Is Valid`
          (`KismetSystemLibrary.PrintString` (`KismetSystemLibrary.GetDisplayName` _returnvalue)))
        (:`Is Not Valid`
          (`KismetSystemLibrary.PrintString` "Owner is Null"))))))

(event `/Game/Utility/BPI_OnOff.Activate`
  (`self.InitStatus`))

(event `InputAction|LockOn`
  (params (Key :type "Key Structure"))
  ; Lock On/Off
  (:`Pressed`
    (if (`self.LockedOn?`)
      (set `self.LockedOn?` false)
      (else
        (set `self.LockedOn?` true)))))

(event `self.ReceiveTick`
  (params (DeltaSeconds :type "Float (single-precision)"))
  (bind _bossactor (`self.BossActor`))
  (bind _bossactor_2 (`self.BossActor`))
  (bind _capsulecomponent (`self.CapsuleComponent`))
  (bind _capsulecomponent_2 (`self.CapsuleComponent`))
  (bind _returnvalue (`SceneComponent.K2_GetComponentLocation` _capsulecomponent_2))
  (bind _returnvalue_2 (`SceneComponent.K2_GetComponentLocation` (`Actor.RootComponent` _bossactor_2)))
  (bind _returnvalue_3 (`KismetMathLibrary.MakeRotFromX` (- (`KismetMathLibrary.MakeVector` (.x _returnvalue_2) (.y _returnvalue_2) (.z _returnvalue_2)) _returnvalue)))
  (bind _yaw (.yaw _returnvalue_3))
  (bind _asbp_souls_game_instance (cast `/Game/Blueprints/BP_SoulsGameInstance` (`GameplayStatics.GetGameInstance`)))
  (if (`|EnumEquality` (`/Game/Blueprints/BP_SoulsGameInstance.CurrentGameState` _asbp_souls_game_instance) "NewEnumerator2")
    (`self.GetInGameUI`)
    (if (< (`self.CurrentHP`) 0.0)
      (if (not (`self.Dead?`))
        (set `self.Dead?` true)
        ; Display You Die
        (`self.PlayAnimMontage` "/Game/Player/Animations/Montages/PlayerDead_AnimMontage.PlayerDead_AnimMontage")
        (bind _asbp_souls_game_instance_2 (cast `/Game/Blueprints/BP_SoulsGameInstance` (`GameplayStatics.GetGameInstance`)))
        (`/Game/Blueprints/BP_SoulsGameInstance.ChangeState` _asbp_souls_game_instance_2 "NewEnumerator3" false))
      (else
        (`/Engine/EditorBlueprintResources/StandardMacros.IsValid` _bossactor
          (:`Is Valid`
            _)
          (:`Is Not Valid`
            _))
        (if (> (`self.DistanceBetweenPlayer` _bossactor) 1750.0)
          (set `self.LockedOn?` false))
        (if (not (`self.BlockPressed?`))
          (`self.StopAnimMontage` "/Game/Player/Animations/Montages/Block_AnimMontage.Block_AnimMontage"))
        (if (`self.LockedOn?`)
          ; Locked On
          (`/Engine/EditorBlueprintResources/StandardMacros.IsValid` _bossactor_2
            (:`Is Valid`
              (set `self.CameraBasedMovementRotation` _returnvalue_3)
              (if (`self.Blocked?`)
                (`SceneComponent.K2_SetWorldRotation` _capsulecomponent_2 (`KismetMathLibrary.MakeRotator` 0.0 0.0 _yaw) false false :!label _label)
                (elif (`self.Rolling?`)
                  _
                  (elif (`self.RollPressed?`)
                    _
                    (else
                      (goto _label)))))
              (`Controller.SetControlRotation` (`self.GetController`) (`KismetMathLibrary.MakeRotator` 0.0 (+ (`KismetMathLibrary.Lerp` -50.0 -15.0 (`KismetMathLibrary.SafeDivide` (`KismetMathLibrary.Vector_Distance` _returnvalue_2 _returnvalue) 1750.0)) (.pitch _returnvalue_3)) _yaw)))
            (:`Is Not Valid`
              _)))
        (if (`self.Backstepping?`)
          ; Backstep (Moving Location)
          (set `self.CanAct?` false)
          (if (`self.LockedOn?`)
            (`SceneComponent.K2_SetWorldRotation` (`self.CapsuleComponent`) _returnvalue_3 false false))
          (`SceneComponent.K2_SetWorldLocation` _capsulecomponent (+ (`SceneComponent.K2_GetComponentLocation` _capsulecomponent) (* (`SceneComponent.GetForwardVector` (`self.ArrowComp`)) (-9.0 -9.0 -9.0))) true false))
        ; Run/Roll/Backstep
        ;; Run
        (if (`self.RollPressed?`)
          (if (not (`self.Drinking?`))
            (set `self.PressedTime` (+ (`GameplayStatics.GetWorldDeltaSeconds`) (`self.PressedTime`)))
            (if (> (`self.PressedTime`) 0.49)
              (set `CharacterMovementComponent.MaxWalkSpeed` 900.0 (`self.CharacterMovement`)))))))))

(event `InputAction|Dodge/Run/Jump/Backstep`
  (params (Key :type "Key Structure"))
  (bind _charactermovement (`self.CharacterMovement`))
  (bind _charactermaxspeed (`self.CharacterMaxSpeed`))
  (bind _drinking_ (`self.Drinking?`))
  ; Run/Roll/Backstep
  (:`Pressed`
    (if (not _drinking_)
      ;; Roll
      (set `self.RollPressed?` true)
      (set `CharacterMovementComponent.MaxWalkSpeed` (`self.CharacterMaxSpeed`) (`self.CharacterMovement`))))
  (:`Released`
    ;; Backstep Animation
    (if (`self.Moving?`)
      (if _drinking_
        _
        (elif (<= (`self.PressedTime`) 0.26)
          (set `self.RollPressed?` false)
          (set `self.Rolling?` true)
          (set `self.PressedTime` 0.0)
          (set `CharacterMovementComponent.MaxWalkSpeed` _charactermaxspeed _charactermovement)
          (if (`self.CanAct?`)
            (if (`self.LockedOn?`)
              (`self.K2_SetActorRotation` (`self.InputBasedMovementRotation`))
              (else
                (`self.K2_SetActorRotation` (`self.CameraBasedMovementRotation`))))
            (`|PlayMontage` (`self.Mesh`) "/Game/Player/Animations/Montages/Roll_AnimMontage.Roll_AnimMontage"
              (:`then`
                (`KismetSystemLibrary.Delay` 33.0)
                (set `self.Rolling?` false))))
          (else
            (set `self.RollPressed?` false)
            (set `self.PressedTime` 0.0)
            (set `CharacterMovementComponent.MaxWalkSpeed` _charactermaxspeed _charactermovement))))
      (elif (`self.CanAct?`)
        (set `self.Backstepping?` true)
        (`|PlayMontage` (`self.Mesh`) "/Game/Player/Animations/Montages/Backstep_AnimMontage.Backstep_AnimMontage"
          (:`then`
            (`KismetSystemLibrary.Delay` 0.6)
            (set `self.Backstepping?` false)
            (set `self.CanAct?` true)))))))

(event `InputAction|ScrollUp`
  (params (Key :type "Key Structure"))
  ; Scroll Dungeon
  (:`Pressed`
    (if (`self.Resting?`)
      (`/Game/UI/WBP_InGame.HighlightStartDungeon` (`self.InGameUI`))
      (set `self.ExitDungeonSelected?` false))))

(event `InputAxis|MoveForward/Backward`
  (params (AxisValue :type "Float (single-precision)"))
  (bind _yaw (.yaw (`self.GetControlRotation`)))
  ; Character Movement
  (set `self.Moving?` true)
  (bind _returnvalue (`KismetMathLibrary.MakeVector` AxisValue (stale `InputAxis|MoveRight/Left` AxisValue)))
  (if (== _returnvalue (0.0 0.0 0.0))
    (set `self.Moving?` false))
  (if (`self.LockedOn?`)
    (bind _returnvalue_2 (`KismetMathLibrary.MakeRotator` 0.0 0.0 (+ (.yaw (`KismetMathLibrary.MakeRotFromX` _returnvalue)) _yaw)))
    (set `self.InputBasedMovementRotation` _returnvalue_2)
    (else
      (set `self.CameraBasedMovementRotation` _returnvalue_2)))
  (if (`self.Drinking?`)
    (`self.AddMovementInput` (`KismetMathLibrary.GetForwardVector` (`KismetMathLibrary.MakeRotator` 0.0 0.0 _yaw)) AxisValue :!label _label_2)
    (elif (`self.CanAct?`)
      (goto _label_2))))

(event `InputAction|ScrollDOwn`
  (params (Key :type "Key Structure"))
  ; Scroll Dungeon
  (:`Pressed`
    (if (`self.Resting?`)
      (`/Game/UI/WBP_InGame.HighlightEndDungeon` (`self.InGameUI`))
      (set `self.ExitDungeonSelected?` true))))

(event `InputAction|Attack(Righthand)`
  (params (Key :type "Key Structure"))
  (bind _bossactor (`self.BossActor`))
  ; Light Attack (Right Hand)
  (:`Pressed`
    (if (== (`self.ComboState`) 1)
      (if (`self.Moving?`)
        (`self.K2_SetActorRotation` (`self.CameraBasedMovementRotation`)))
      (`|PlayMontage` (`self.Mesh`) "/Game/Player/Animations/Montages/LightAttack1_AnimMontage.LightAttack1_AnimMontage")
      (elif (== (`self.ComboState`) 2)
        (if (`self.Moving?`)
          (`self.K2_SetActorRotation` (`self.CameraBasedMovementRotation`)))
        (`|PlayMontage` (`self.Mesh`) "/Game/Player/Animations/Montages/LightAttack2_AnimMontage.LightAttack2_AnimMontage")
        (elif (`self.CanAct?`)
          (`/Engine/EditorBlueprintResources/StandardMacros.IsValid` _bossactor
            (:`Is Valid`
              (if (`/Game/Boss/Character/BP_Boss.SendGroggyState` _bossactor)
                (bind (_location _rotator) (`/Game/Boss/Character/BP_Boss.PullTargetFrontOfBoss` (`self.BossActor`)))
                (`self.K2_SetActorLocationAndRotation` (`KismetMathLibrary.MakeVector` (.x _location) (.y _location) (- (.z _location) 100.0)) _rotator true)
                (`|PlayMontage` (`self.Mesh`) "/Game/Player/Animations/Montages/CriticalAttack_AnimMontage.CriticalAttack_AnimMontage")
                (else
                  (if (`self.Moving?`)
                    (`self.K2_SetActorRotation` (`self.CameraBasedMovementRotation`)))
                  (`|PlayMontage` (`self.Mesh`) "/Game/Player/Animations/Montages/LightAttack0_AnimMontage.LightAttack0_AnimMontage"))))))))))

(event `InputAxis|MoveRight/Left`
  (params (AxisValue :type "Float (single-precision)"))
  (bind _yaw (.yaw (`self.GetControlRotation`)))
  ; Character Movement
  (set `self.Moving?` true)
  (bind _returnvalue (`KismetMathLibrary.MakeVector` (stale `InputAxis|MoveForward/Backward` AxisValue) AxisValue))
  (if (== _returnvalue (0.0 0.0 0.0))
    (set `self.Moving?` false))
  (if (`self.LockedOn?`)
    (bind _returnvalue_2 (`KismetMathLibrary.MakeRotator` 0.0 0.0 (+ (.yaw (`KismetMathLibrary.MakeRotFromX` _returnvalue)) _yaw)))
    (set `self.InputBasedMovementRotation` _returnvalue_2)
    (else
      (set `self.CameraBasedMovementRotation` _returnvalue_2)))
  (if (`self.Drinking?`)
    (`self.AddMovementInput` (`KismetMathLibrary.GetRightVector` (`KismetMathLibrary.MakeRotator` 0.0 0.0 _yaw)) AxisValue :!label _label_3)
    ;; Player followed Camera (when moving left/right)
    (`self.AddControllerYawInput` (* AxisValue 0.21))
    (elif (`self.CanAct?`)
      (goto _label_3))))

(event `InputAction|UseItem`
  (params (Key :type "Key Structure"))
  (:`Pressed`
    (if (`self.CanAct?`)
      (`|PlayMontage` (`self.Mesh`) "/Game/Player/Animations/Montages/Drinking_AnimMontage.Drinking_AnimMontage"))))

(event `InputAxis|LookUp/Down`
  (params (AxisValue :type "Float (single-precision)"))
  ; Camera Movement
  ;; Look Up (Pitch)
  (if (`self.CriticalAttacking?`)
    _
    (elif (not (`self.LockedOn?`))
      (set `SpringArmComponent.CameraRotationLagSpeed` 0.0 (`self.SpringArmComp`))
      (`self.AddControllerPitchInput` AxisValue)
      (if (== (+ (`self.GetInputAxisValue`) (`self.GetInputAxisValue`)) 0.0)
        (set `SpringArmComponent.CameraRotationLagSpeed` 4.0 (`self.SpringArmComp`))))))

(event `InputAction|Interaction`
  (params (Key :type "Key Structure"))
  (bind _door (`self.Door`))
  (bind _ingameui (`self.InGameUI`))
  (:`Pressed`
    (`/Engine/EditorBlueprintResources/StandardMacros.IsValid` _door
      (:`Is Valid`
        (message `/Game/Utility/BPI_Stuff.Interact` _door))
      (:`Is Not Valid`
        ; 보스 화톳불 상호작용시 메인메뉴로
        (if (`/Game/Boss/Character/Status/StatusComp.IsDead` (`/Game/Boss/Character/BP_Boss.StatusComp` (`self.BossActor`)))
          (if (`self.CanAct?`)
            (`|PlayMontage` (`self.Mesh`) "/Game/Player/Animations/Montages/LitBonfire_AnimMontage.LitBonfire_AnimMontage"
              (:`then`
                (`KismetSystemLibrary.Delay` 3.0)
                ; 화톳불 점화
                (bind _asbp_soul_game_mode_level_and_state (cast `/Game/Blueprints/BP_SoulGameMode_LevelAndState` (`GameplayStatics.GetGameMode`)))
                (`/Game/Blueprints/BP_SoulGameMode_LevelAndState.ChangeStateWithLoading` _asbp_soul_game_mode_level_and_state "NewEnumerator0"))))
          (else
            ; 게임 종료 시
            (if (`self.ExitDungeonSelected?`)
              (bind _asbp_souls_game_instance (cast `/Game/Blueprints/BP_SoulsGameInstance` (`GameplayStatics.GetGameInstance`)))
              (`/Game/Blueprints/BP_SoulsGameInstance.ChangeState` _asbp_souls_game_instance "NewEnumerator0" true)
              (elif (`self.InteractionDisabled?`)
                _
                (elif (`/Game/Stuff/bonfire/BP_Bonfire.RestingAvailable?` (`self.BonfireActor`))
                  (if (`self.Resting?`)
                    (`|PlayMontage` (`self.Mesh`) "/Game/Player/Animations/Montages/Stand_AnimMontage.Stand_AnimMontage"
                      (:`then`
                        (set `self.Resting?` false)
                        (`/Game/UI/WBP_InGame.DungeonNameInvisible` _ingameui)))
                    (else
                      (`|PlayMontage` (`self.Mesh`) "/Game/Player/Animations/Montages/Sit_AnimMontage.Sit_AnimMontage"
                        (:`then`
                          (set `self.Resting?` true)
                          (`/Game/UI/WBP_InGame.DungeonNameVisible` _ingameui)
                          (bind _asbp_soul_game_mode_level_and_state_2 (cast `/Game/Blueprints/BP_SoulGameMode_LevelAndState` (`GameplayStatics.GetGameMode`)))
                          (`/Game/Blueprints/BP_SoulGameMode_LevelAndState.ResetBossLevel` _asbp_soul_game_mode_level_and_state_2))))))))))))))

(event `InputAxis|TurnRight/Left`
  (params (AxisValue :type "Float (single-precision)"))
  ; Camera Movement
  ;; Turn (Yaw)
  (if (`self.CriticalAttacking?`)
    _
    (elif (not (`self.LockedOn?`))
      (set `SpringArmComponent.CameraRotationLagSpeed` 0.0 (`self.SpringArmComp`))
      (`self.AddControllerYawInput` AxisValue)
      (if (== (+ (`self.GetInputAxisValue`) (`self.GetInputAxisValue`)) 0.0)
        (set `SpringArmComponent.CameraRotationLagSpeed` 4.0 (`self.SpringArmComp`))))))

(event `InputAction|StrongAttack(LeftHand)`
  (params (Key :type "Key Structure"))
  ; Strong Attack (Left Hand, Parry)
  (:`Pressed`
    (if (`self.CanAct?`)
      (if (`self.LockedOn?`)
        (`self.K2_SetActorRotation` (`self.CameraBasedMovementRotation`)))
      (`|PlayMontage` (`self.Mesh`) "/Game/Player/Animations/Montages/Parry_AnimMontage.Parry_AnimMontage"))))

(event `InputAction|Attack(LeftHand)`
  (params (Key :type "Key Structure"))
  ; Light Attack (left Hand, Block)
  (:`Pressed`
    (set `self.BlockPressed?` true)
    (`self.Block` :!label _label_4))
  (:`Released`
    (set `self.BlockPressed?` false)))

(event `KeepBlocking`
  ; Light Attack (left Hand, Block)
  (goto _label_4))

(fn `Block`
  (if (`self.CanAct?`)
    (`self.K2_SetActorRotation` (`self.CameraBasedMovementRotation`))
    (`self.PlayAnimMontage` "/Game/Player/Animations/Montages/Block_AnimMontage.Block_AnimMontage")))

(fn `DistanceBetweenPlayer`
  (params (InputActor :type "Actor Object Reference"))
  (returns (Distance :type "Float (double-precision)"))
  (return (`self.GetDistanceTo` InputActor (`GameplayStatics.GetPlayerPawn` 0))))

(fn `GetInGameUI`
  (`/Engine/EditorBlueprintResources/StandardMacros.IsValid` (`self.InGameUI`)
    (:`Is Valid`
      _)
    (:`Is Not Valid`
      (bind _asbp_soul_game_mode_level_and_state (cast `/Game/Blueprints/BP_SoulGameMode_LevelAndState` (`GameplayStatics.GetGameMode`)))
      (set `self.InGameUI` (`/Game/UI/BP_HUD_LevelAndState.InGame` (`/Game/Blueprints/BP_SoulGameMode_LevelAndState.OurHud` _asbp_soul_game_mode_level_and_state)))))
  (return))

(fn `IgnoreRootMotion`
  (params (ignore :type Boolean))
  (bind _returnvalue (`SkeletalMeshComponent.GetAnimInstance` (`self.Mesh`)))
  (if ignore
    (`AnimInstance.SetRootMotionMode` _returnvalue "IgnoreRootMotion")
    (else
      (`AnimInstance.SetRootMotionMode` _returnvalue "RootMotionFromEverything"))))

(fn `InGameStandingMotion`
  (`self.PlayAnimMontage` "/Game/Player/Animations/Montages/Stand_AnimMontage.Stand_AnimMontage"))

(fn `InitStatus`
  (set `self.CurrentHP` (`self.MaxHP`))
  (set `self.EstusAmount` (`self.MaxEstusAmount`)))

(fn `IsPlayerLooking`
  (params (InputActor :type "Actor Object Reference"))
  (returns (`Looking?` :type Boolean))
  (bind _returnvalue (`GameplayStatics.GetPlayerPawn` 0))
  (if (> (`KismetMathLibrary.Dot_VectorVector` (- (`self.K2_GetActorLocation` InputActor) (`self.K2_GetActorLocation` _returnvalue)) (`KismetMathLibrary.GetForwardVector` (`self.K2_GetActorRotation` _returnvalue))) 0.0)
    (return true)
    (else
      (return false))))

(fn `PlayerDamaged`
  (params (DamageValue :type "Float (double-precision)"))
  (if (`self.Invincible?`)
    _
    (elif (> DamageValue 0.0)
      (if (`self.Dead?`)
        _
        (elif (`self.Blocked?`)
          (bind _returnvalue (`self.PlayAnimMontage` "/Game/Player/Animations/Montages/Blocked_AnimMontage.Blocked_AnimMontage"))
          (set `self.CurrentHP` (- (`self.CurrentHP`) (* (`local.DamageValue`) 0.4)))
          (`KismetSystemLibrary.K2_SetTimerDelegate` (`|CreateDelegate` :!event `KeepBlocking`) _returnvalue)
          (else
            (`self.PlayAnimMontage` "/Game/Player/Animations/Montages/Flinch_AnimMontage.Flinch_AnimMontage")
            (set `self.CurrentHP` (- (`self.CurrentHP`) (`local.DamageValue`)))))))))

(fn `SendHP`
  (returns (HP :type "/Game/Utility/F_ConsumableValue Structure"))
  (return))

(fn `UserConstructionScript`)